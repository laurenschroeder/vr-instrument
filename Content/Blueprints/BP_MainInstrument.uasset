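; VR musical instrument that turns a motion controller's position into live MetaSound synth parameters.
; Tick measures ActiveController, which this graph never assigns, against marker spheres: Z drives a one-octave note, X gain, Y flanger.
; Triangle, Square and Sine overlaps select the waveform and highlight its button.
; BeginPlay attaches particles to both VRPTPawn controllers; Box and FlyBox overlaps set material distortion, with FlyBox also playing a sound.
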(event `self.ReceiveBeginPlay`
  ;[1 1 1] Initialize Emitters
  (bind _returnvalue (`GameplayStatics.GetActorOfClass` "/Game/Passthrough/Blueprints/VRPTPawn.VRPTPawn_C"))
  (`GameplayStatics.SpawnEmitterAttached` "/Engine/Tutorial/SubEditors/TutorialAssets/TutorialParticleSystem.TutorialParticleSystem" (`/Game/Passthrough/Blueprints/VRPTPawn.MotionControllerLeft` _returnvalue) "None" (0.0 0.0 0.0) (struct) (0.3 0.3 0.3))
  (`GameplayStatics.SpawnEmitterAttached` "/Engine/Tutorial/SubEditors/TutorialAssets/TutorialParticleSystem.TutorialParticleSystem" (`/Game/Passthrough/Blueprints/VRPTPawn.MotionControllerRight` _returnvalue) "None" (0.0 0.0 0.0) (struct) (0.3 0.3 0.3)))

(event `self.ReceiveTick`
  (params (DeltaSeconds :type "Float (single-precision)"))
  (bind _activecontroller (`self.activeController`))
  (bind _newmetasoundsource (`self.NewMetaSoundSource`))
  (bind (_returnvalue_x _returnvalue_y) (`KismetMathLibrary.BreakVector` (`SceneComponent.K2_GetComponentLocation` (`self.YSphere`))))
  (bind (_returnvalue_x_2 _returnvalue_y_2 _returnvalue_z) (`KismetMathLibrary.BreakVector` (`SceneComponent.K2_GetComponentLocation` _activecontroller)))
  (bind (_returnvalue_x_3 _returnvalue_y_3 _returnvalue_z_2) (`KismetMathLibrary.BreakVector` (`SceneComponent.K2_GetComponentLocation` (`self.OriginSphere`))))
  (bind (_returnvalue_x_4 _returnvalue_y_4 _returnvalue_z_3) (`KismetMathLibrary.BreakVector` (`SceneComponent.K2_GetComponentLocation` (`self.ZSphere`))))
  ;[1 1 1] Initialize Emitters
  (`KismetSystemLibrary.PrintString` (`KismetSystemLibrary.GetDisplayName` _activecontroller) false false)
  (if (!= _activecontroller (`self.emptyController`))
    (`AudioParameterControllerInterface.SetFloatParameter` _newmetasoundsource "ScaleNote" (`KismetMathLibrary.MapRangeClamped` (/ (- _returnvalue_z_3 _returnvalue_z) (- _returnvalue_z_3 _returnvalue_z_2)) 1.0 0.0 60.0 72.0))
    (`AudioParameterControllerInterface.SetFloatParameter` _newmetasoundsource "Gain0" (`KismetMathLibrary.MapRangeClamped` (`KismetMathLibrary.Abs` (- _returnvalue_x_3 _returnvalue_x_2)) 25.0 0.0 0.0 1.0))
    (`AudioParameterControllerInterface.SetFloatParameter` _newmetasoundsource "Flanger" (* (/ (- _returnvalue_y _returnvalue_y_2) (- _returnvalue_y _returnvalue_y_3)) 8.0))))

(event `self.Box.OnComponentBeginOverlap`
  (params (OverlappedComponent :type "PrimitiveComponent Object Reference") (OtherActor :type "Actor Object Reference") (OtherComp :type "PrimitiveComponent Object Reference") (OtherBodyIndex :type Integer) (bFromSweep :type Boolean) (SweepResult :type "HitResult Structure (by ref)"))
  (if (not (`self.isOverlapping`))
    (`MeshComponent.SetScalarParameterValueOnMaterials` (`self.Triangle`) "DistortionOn" 1.0)
    (set `self.isOverlapping` true)))

(event `self.Box.OnComponentEndOverlap`
  (params (OverlappedComponent :type "PrimitiveComponent Object Reference") (OtherActor :type "Actor Object Reference") (OtherComp :type "PrimitiveComponent Object Reference") (OtherBodyIndex :type Integer))
  (`MeshComponent.SetScalarParameterValueOnMaterials` (`self.Triangle`) "DistortionOn" 1.0)
  (set `self.isOverlapping` false))

(event `self.FlyBox.OnComponentBeginOverlap`
  (params (OverlappedComponent :type "PrimitiveComponent Object Reference") (OtherActor :type "Actor Object Reference") (OtherComp :type "PrimitiveComponent Object Reference") (OtherBodyIndex :type Integer) (bFromSweep :type Boolean) (SweepResult :type "HitResult Structure (by ref)"))
  (bind _fly (`self.Fly`))
  (`MeshComponent.SetScalarParameterValueOnMaterials` _fly "DistortionOn" 1.0)
  (`GameplayStatics.PlaySoundAtLocation` "/Game/Sounds/ufx2_noisedirt_010.ufx2_noisedirt_010" (`SceneComponent.K2_GetComponentLocation` _fly) (struct) 1.0 1.0 0.0 null null null null))

(event `self.Fly.OnComponentBeginOverlap`
  (params (OverlappedComponent :type "PrimitiveComponent Object Reference") (OtherActor :type "Actor Object Reference") (OtherComp :type "PrimitiveComponent Object Reference") (OtherBodyIndex :type Integer) (bFromSweep :type Boolean) (SweepResult :type "HitResult Structure (by ref)")))

(event `self.FlyBox.OnComponentEndOverlap`
  (params (OverlappedComponent :type "PrimitiveComponent Object Reference") (OtherActor :type "Actor Object Reference") (OtherComp :type "PrimitiveComponent Object Reference") (OtherBodyIndex :type Integer))
  (`MeshComponent.SetScalarParameterValueOnMaterials` (`self.Fly`) "DistortionOn" 0.0))

(event `self.Triangle.OnComponentBeginOverlap`
  (params (OverlappedComponent :type "PrimitiveComponent Object Reference") (OtherActor :type "Actor Object Reference") (OtherComp :type "PrimitiveComponent Object Reference") (OtherBodyIndex :type Integer) (bFromSweep :type Boolean) (SweepResult :type "HitResult Structure (by ref)"))
  ;[1 1 1] Change Waveform Buttons
  (`AudioParameterControllerInterface.SetFloatParameter` (`self.NewMetaSoundSource`) "WaveType" 0.0)
  (`self.ResetButtons` (`self.defaultMaterial`))
  (`PrimitiveComponent.SetMaterial` (`self.ButtonTri`) 0 "/Engine/VREditor/UI/ArrowMaterial.ArrowMaterial"))

(event `self.Square.OnComponentBeginOverlap`
  (params (OverlappedComponent :type "PrimitiveComponent Object Reference") (OtherActor :type "Actor Object Reference") (OtherComp :type "PrimitiveComponent Object Reference") (OtherBodyIndex :type Integer) (bFromSweep :type Boolean) (SweepResult :type "HitResult Structure (by ref)"))
  ;[1 1 1] Change Waveform Buttons
  (`AudioParameterControllerInterface.SetFloatParameter` (`self.NewMetaSoundSource`) "WaveType" 1.0)
  (`self.ResetButtons` (`self.defaultMaterial`))
  (`PrimitiveComponent.SetMaterial` (`self.ButtonSquare`) 0 "/Engine/VREditor/UI/ArrowMaterial.ArrowMaterial"))

(event `self.Sine.OnComponentBeginOverlap`
  (params (OverlappedComponent :type "PrimitiveComponent Object Reference") (OtherActor :type "Actor Object Reference") (OtherComp :type "PrimitiveComponent Object Reference") (OtherBodyIndex :type Integer) (bFromSweep :type Boolean) (SweepResult :type "HitResult Structure (by ref)"))
  ;[1 1 1] Change Waveform Buttons
  (`AudioParameterControllerInterface.SetFloatParameter` (`self.NewMetaSoundSource`) "WaveType" 2.0)
  (`self.ResetButtons` (`self.defaultMaterial`))
  (`PrimitiveComponent.SetMaterial` (`self.ButtonSine`) 0 "/Engine/VREditor/UI/ArrowMaterial.ArrowMaterial"))

(fn `ResetButtons`
  (params (DefaultMaterial :type "Material Object Reference"))
  (`PrimitiveComponent.SetMaterial` (`self.ButtonSquare`) 0 DefaultMaterial)
  (`PrimitiveComponent.SetMaterial` (`self.ButtonSine`) 0 DefaultMaterial)
  (`PrimitiveComponent.SetMaterial` (`self.ButtonTri`) 0 DefaultMaterial))

(fn `UserConstructionScript`)
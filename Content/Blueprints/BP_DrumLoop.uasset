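; BP_DrumLoop is an interactive drum loop switcher driven by overlaps with floppy components.
; BeginPlay spawns a persistent 2D sound; the Berp, Yay and Ahh floppies swap its loop and toggle it active if IsPlaying is false.
; The Neutral floppy toggles it off when IsPlaying is true.
; A DistortionOn material parameter highlights the selected floppy, cleared through FloppysOff, and mirrors IsPlaying on DrumPlane whenever playback toggles.
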(event `self.ReceiveBeginPlay`
  (bind _returnvalue (`GameplayStatics.SpawnSound2D` (`self.Sound`) 1.0 1.0 0.0 null false false)))

(event `self.Box.OnComponentBeginOverlap`
  (params (OverlappedComponent :type "PrimitiveComponent Object Reference") (OtherActor :type "Actor Object Reference") (OtherComp :type "PrimitiveComponent Object Reference") (OtherBodyIndex :type Integer) (bFromSweep :type Boolean) (SweepResult :type "HitResult Structure (by ref)")))

(event `self.NeutralFloppy.OnComponentBeginOverlap`
  (params (OverlappedComponent :type "PrimitiveComponent Object Reference") (OtherActor :type "Actor Object Reference") (OtherComp :type "PrimitiveComponent Object Reference") (OtherBodyIndex :type Integer) (bFromSweep :type Boolean) (SweepResult :type "HitResult Structure (by ref)"))
  (if (`self.isPlaying`)
    (`self.FloppysOff`)
    (`MeshComponent.SetScalarParameterValueOnMaterials` (`self.NeutralFloppy`) "DistortionOn" 1.0)
    (`ActorComponent.ToggleActive` (stale `self.ReceiveBeginPlay` _returnvalue) :!label _label)
    (bind _output_get (set `self.isPlaying` (not (`self.isPlaying`))))
    (`MeshComponent.SetScalarParameterValueOnMaterials` (`self.DrumPlane`) "DistortionOn" (`KismetMathLibrary.Conv_BoolToDouble` _output_get))))

(event `self.BerpFloppy.OnComponentBeginOverlap`
  (params (OverlappedComponent :type "PrimitiveComponent Object Reference") (OtherActor :type "Actor Object Reference") (OtherComp :type "PrimitiveComponent Object Reference") (OtherBodyIndex :type Integer) (bFromSweep :type Boolean) (SweepResult :type "HitResult Structure (by ref)"))
  (`AudioComponent.SetSound` (stale `self.ReceiveBeginPlay` _returnvalue) "/Game/Sounds/Loops/Drums/NW_NDRE_90_drum_daytona_full.NW_NDRE_90_drum_daytona_full")
  (`self.FloppysOff`)
  (`MeshComponent.SetScalarParameterValueOnMaterials` (`self.BerpFloppy`) "DistortionOn" 1.0)
  (if (not (`self.isPlaying`)) :!label _label_2
    (goto _label)))

(event `self.YayFloppy.OnComponentBeginOverlap`
  (params (OverlappedComponent :type "PrimitiveComponent Object Reference") (OtherActor :type "Actor Object Reference") (OtherComp :type "PrimitiveComponent Object Reference") (OtherBodyIndex :type Integer) (bFromSweep :type Boolean) (SweepResult :type "HitResult Structure (by ref)"))
  (`AudioComponent.SetSound` (stale `self.ReceiveBeginPlay` _returnvalue) "/Game/Sounds/Loops/Drums/NW_NTPS_90_drum_sundiver_full.NW_NTPS_90_drum_sundiver_full")
  (`self.FloppysOff`)
  (`MeshComponent.SetScalarParameterValueOnMaterials` (`self.YayFloppy`) "DistortionOn" 1.0)
  (goto _label_2))

(event `self.Ahh_Floppy.OnComponentBeginOverlap`
  (params (OverlappedComponent :type "PrimitiveComponent Object Reference") (OtherActor :type "Actor Object Reference") (OtherComp :type "PrimitiveComponent Object Reference") (OtherBodyIndex :type Integer) (bFromSweep :type Boolean) (SweepResult :type "HitResult Structure (by ref)"))
  (`AudioComponent.SetSound` (stale `self.ReceiveBeginPlay` _returnvalue) "/Game/Sounds/Loops/Drums/SS_NC_90_Drum_BoopBoop_Full.SS_NC_90_Drum_BoopBoop_Full")
  (`self.FloppysOff`)
  (`MeshComponent.SetScalarParameterValueOnMaterials` (`self.Ahh_Floppy`) "DistortionOn" 1.0)
  (goto _label_2))

(fn `FloppysOff`
  (`MeshComponent.SetScalarParameterValueOnMaterials` (`self.Ahh_Floppy`) "DistortionOn" 0.0)
  (`MeshComponent.SetScalarParameterValueOnMaterials` (`self.BerpFloppy`) "DistortionOn" 0.0)
  (`MeshComponent.SetScalarParameterValueOnMaterials` (`self.NeutralFloppy`) "DistortionOn" 0.0)
  (`MeshComponent.SetScalarParameterValueOnMaterials` (`self.YayFloppy`) "DistortionOn" 0.0))

(fn `ToggleSoundPlaying`)

(fn `UserConstructionScript`)
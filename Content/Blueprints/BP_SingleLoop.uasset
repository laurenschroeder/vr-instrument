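; BP_SingleLoop is an actor that toggles a 2D sound on and off whenever something begins overlapping its Box.
; BeginPlay spawns the sound without auto-destroy and immediately runs the same toggle once.
; Each toggle flips the audio component's active state and IsPlaying, then sets DrumPlane's DistortionOn material parameter to the inverse of IsPlaying.
; The construction script applies the Icon material to DrumPlane.
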(event `self.ReceiveBeginPlay`
  (bind _returnvalue (`GameplayStatics.SpawnSound2D` (`self.Sound`) 1.0 1.0 0.0 null false false))
  (`ActorComponent.ToggleActive` _returnvalue :!label _label)
  (bind _output_get (set `self.isPlaying` (not (`self.isPlaying`))))
  (`MeshComponent.SetScalarParameterValueOnMaterials` (`self.DrumPlane`) "DistortionOn" (`KismetMathLibrary.Conv_BoolToDouble` (not _output_get))))

(event `self.Box.OnComponentBeginOverlap`
  (params (OverlappedComponent :type "PrimitiveComponent Object Reference") (OtherActor :type "Actor Object Reference") (OtherComp :type "PrimitiveComponent Object Reference") (OtherBodyIndex :type Integer) (bFromSweep :type Boolean) (SweepResult :type "HitResult Structure (by ref)"))
  (goto _label))

(fn `UserConstructionScript`
  (`PrimitiveComponent.SetMaterial` (`self.DrumPlane`) 0 (`self.Icon`)))
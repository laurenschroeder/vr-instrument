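; VR spatial instrument that turns the position of the pawn's right motion controller into MetaSound parameters.
; Entering the Box stores that controller, attaches a particle effect and enables plane distortion; leaving does not clear the controller.
; While TriggerOn is set, Tick measures it against marker spheres, with Z driving a one-octave ScaleNote and X and Y driving two gains; otherwise Gain0 is muted.
; A separate Fly component distorts and plays a sound on overlap.
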(event `self.ReceiveTick`
  (params (DeltaSeconds :type "Float (single-precision)"))
  (bind _newmetasoundsource (`self.NewMetaSoundSource`))
  (bind _activecontroller (`self.activeController`))
  (bind (_returnvalue_x _returnvalue_y) (`KismetMathLibrary.BreakVector` (`SceneComponent.K2_GetComponentLocation` (`self.YSphere`))))
  (bind (_returnvalue_x_2 _returnvalue_y_2 _returnvalue_z) (`KismetMathLibrary.BreakVector` (`SceneComponent.K2_GetComponentLocation` _activecontroller)))
  (bind (_returnvalue_x_3 _returnvalue_y_3 _returnvalue_z_2) (`KismetMathLibrary.BreakVector` (`SceneComponent.K2_GetComponentLocation` (`self.OriginSphere`))))
  (bind (_returnvalue_x_4 _returnvalue_y_4 _returnvalue_z_3) (`KismetMathLibrary.BreakVector` (`SceneComponent.K2_GetComponentLocation` (`self.ZSphere`))))
  (bind _returnvalue (`KismetMathLibrary.Abs` (- _returnvalue_x_3 _returnvalue_x_2)))
  (bind _returnvalue_2 (/ (- _returnvalue_z_3 _returnvalue_z) (- _returnvalue_z_3 _returnvalue_z_2)))
  (bind _returnvalue_3 (/ (- _returnvalue_y _returnvalue_y_2) (- _returnvalue_y _returnvalue_y_3)))
  (bind _returnvalue_4 (`KismetMathLibrary.MapRangeClamped` _returnvalue_2 1.0 0.0 60.0 72.0))
  (if (!= _activecontroller (`self.emptyController`))
    (if (`self.triggerOn`)
      (`KismetSystemLibrary.PrintString` (`KismetStringLibrary.Concat_StrStr` "X " (`KismetStringLibrary.Conv_DoubleToString` _returnvalue) " Y " (`KismetStringLibrary.Conv_DoubleToString` _returnvalue_3) " Z " (`KismetStringLibrary.Conv_DoubleToString` _returnvalue_2) "pitch" (`KismetStringLibrary.Conv_DoubleToString` _returnvalue_4)) false false)
      (`AudioParameterControllerInterface.SetFloatParameter` _newmetasoundsource "ScaleNote" _returnvalue_4)
      (`AudioParameterControllerInterface.SetFloatParameter` _newmetasoundsource "Gain0" (`KismetMathLibrary.MapRangeClamped` _returnvalue 25.0 0.0 0.0 1.0))
      (`AudioParameterControllerInterface.SetFloatParameter` _newmetasoundsource "Gain1" _returnvalue_3)
      (else
        (`AudioParameterControllerInterface.SetFloatParameter` _newmetasoundsource "Gain0" 0.0)))))

(event `self.Box.OnComponentBeginOverlap`
  (params (OverlappedComponent :type "PrimitiveComponent Object Reference") (OtherActor :type "Actor Object Reference") (OtherComp :type "PrimitiveComponent Object Reference") (OtherBodyIndex :type Integer) (bFromSweep :type Boolean) (SweepResult :type "HitResult Structure (by ref)"))
  (if (not (`self.isOverlapping`))
    (bind _asvrptpawn (cast `/Game/Passthrough/Blueprints/VRPTPawn` OtherActor))
    (`MeshComponent.SetScalarParameterValueOnMaterials` (`self.MainPlane`) "DistortionOn" 1.0)
    (bind _motioncontrollerright (`/Game/Passthrough/Blueprints/VRPTPawn.MotionControllerRight` _asvrptpawn))
    (`GameplayStatics.SpawnEmitterAttached` "/Engine/Tutorial/SubEditors/TutorialAssets/TutorialParticleSystem.TutorialParticleSystem" _motioncontrollerright "None" (0.0 0.0 0.0) (struct) (0.3 0.3 0.3))
    (set `self.activeController` _motioncontrollerright)
    (set `self.isOverlapping` true)))

(event `self.Box.OnComponentEndOverlap`
  (params (OverlappedComponent :type "PrimitiveComponent Object Reference") (OtherActor :type "Actor Object Reference") (OtherComp :type "PrimitiveComponent Object Reference") (OtherBodyIndex :type Integer))
  (cast `/Game/Passthrough/Blueprints/VRPTPawn` OtherActor)
  (`MeshComponent.SetScalarParameterValueOnMaterials` (`self.MainPlane`) "DistortionOn" 1.0)
  (set `self.isOverlapping` false))

(event `self.Fly.OnComponentBeginOverlap`
  (params (OverlappedComponent :type "PrimitiveComponent Object Reference") (OtherActor :type "Actor Object Reference") (OtherComp :type "PrimitiveComponent Object Reference") (OtherBodyIndex :type Integer) (bFromSweep :type Boolean) (SweepResult :type "HitResult Structure (by ref)"))
  (bind _fly (`self.Fly`))
  (`MeshComponent.SetScalarParameterValueOnMaterials` _fly "DistortionOn" 1.0)
  (`GameplayStatics.PlaySoundAtLocation` "/Game/Sounds/ufx2_noisedirt_010.ufx2_noisedirt_010" (`SceneComponent.K2_GetComponentLocation` _fly) (struct) 1.0 1.0 0.0 null null null null))

(event `self.Fly.OnComponentEndOverlap`
  (params (OverlappedComponent :type "PrimitiveComponent Object Reference") (OtherActor :type "Actor Object Reference") (OtherComp :type "PrimitiveComponent Object Reference") (OtherBodyIndex :type Integer))
  (`MeshComponent.SetScalarParameterValueOnMaterials` (`self.Fly`) "DistortionOn" 0.0))

(fn `UserConstructionScript`)